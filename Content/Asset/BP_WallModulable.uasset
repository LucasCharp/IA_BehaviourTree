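; Modular wall actor that picks its surface look from a WallType setting.
; On BeginPlay, a switch on WallType applies one of eight wall material instances to the first material slot of both static mesh components.
; The construction script is empty, so this material choice is only applied at runtime.
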(event EventBeginPlay
  (bind _staticmesh1 (Variables|Default|GetStaticMesh1))
  (bind _staticmesh (Variables|Default|GetStaticMesh))
  (switch int (Variables|Default|GetWallType)
    (:1
      (Rendering|Material|SetMaterial _staticmesh 0 "/Game/Asset/MI_Wall1.MI_Wall1")
      (Rendering|Material|SetMaterial _staticmesh1 0 "/Game/Asset/MI_Wall1.MI_Wall1"))
    (:2
      (Rendering|Material|SetMaterial _staticmesh 0 "/Game/Asset/MI_Wall2.MI_Wall2")
      (Rendering|Material|SetMaterial _staticmesh1 0 "/Game/Asset/MI_Wall2.MI_Wall2"))
    (:3
      (Rendering|Material|SetMaterial _staticmesh 0 "/Game/Asset/MI_Wall3.MI_Wall3")
      (Rendering|Material|SetMaterial _staticmesh1 0 "/Game/Asset/MI_Wall3.MI_Wall3"))
    (:4
      (Rendering|Material|SetMaterial _staticmesh 0 "/Game/Asset/MI_Wall4.MI_Wall4")
      (Rendering|Material|SetMaterial _staticmesh1 0 "/Game/Asset/MI_Wall4.MI_Wall4"))
    (:5
      (Rendering|Material|SetMaterial _staticmesh 0 "/Game/Asset/MI_Wall5.MI_Wall5")
      (Rendering|Material|SetMaterial _staticmesh1 0 "/Game/Asset/MI_Wall5.MI_Wall5"))
    (:6
      (Rendering|Material|SetMaterial _staticmesh 0 "/Game/Asset/MI_Wall6.MI_Wall6")
      (Rendering|Material|SetMaterial _staticmesh1 0 "/Game/Asset/MI_Wall6.MI_Wall6"))
    (:7
      (Rendering|Material|SetMaterial _staticmesh 0 "/Game/Asset/MI_Wall7.MI_Wall7")
      (Rendering|Material|SetMaterial _staticmesh1 0 "/Game/Asset/MI_Wall7.MI_Wall7"))
    (:8
      (Rendering|Material|SetMaterial _staticmesh 0 "/Game/Asset/MI_Wall8.MI_Wall8")
      (Rendering|Material|SetMaterial _staticmesh1 0 "/Game/Asset/MI_Wall8.MI_Wall8"))))

(fn ConstructionScript)